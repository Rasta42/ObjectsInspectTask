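; Player interaction component that picks which overlapped BPI_Interact actor the owning pawn would interact with.
; Overlap events maintain a candidate list and run a looping sort timer while it has entries.
; CalculateActorWeights ranks candidates by distance plus a heavy penalty for angle off camera forward, measured from an offset right and up of the pawn.
; Only the best actor's marker is enabled, and GetInteractionActor returns it.
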(event Custom|OnActorBeginOverlap_Event
  (params (OverlappedActor :type Actor%20Object%20Reference) (OtherActor :type Actor%20Object%20Reference))
  (if (Utilities|DoesObjectImplementInterface OtherActor "/Game/Prototype/Blueprints/BPI_Interact.BPI_Interact_C")
    (Utilities|Array|AddUnique (Variables|Default|GetOverlappedActors) OtherActor)
    (if (not (Utilities|Time|IsTimerActivebyHandle (Variables|Default|GetSortingTimer)))
      (bind _returnvalue (Utilities|Time|SetTimerbyEvent (EventDispatchers|CreateEvent :!event CalculateActorWeights) 0.1 true true))
      (Variables|Default|SetSortingTimer _returnvalue)
      (CallFunction|CalculateActorWeights))))

(event Custom|OnActorEndOverlap_Event
  (params (OverlappedActor :type Actor%20Object%20Reference) (OtherActor :type Actor%20Object%20Reference))
  (bind _overlappedactors (Variables|Default|GetOverlappedActors))
  (if (Utilities|DoesObjectImplementInterface OtherActor "/Game/Prototype/Blueprints/BPI_Interact.BPI_Interact_C")
    (Class|BPIInteract|SetMarkerState(Message) OtherActor false)
    (Utilities|Array|RemoveItem _overlappedactors OtherActor)
    (if (Utilities|Array|IsEmpty _overlappedactors)
      (Utilities|Time|ClearandInvalidateTimerbyHandle (Variables|Default|GetSortingTimer)))))

(event EventBeginPlay
  (bind _aspawn (Utilities|Casting|CastToPawn (Components|GetOwner)))
  (bind _output_get (Variables|Default|SetPlayer _aspawn))
  (EventDispatchers|AssignOnActorBeginOverlap _output_get (EventDispatchers|CreateEvent :!event Custom|OnActorBeginOverlap_Event))
  (EventDispatchers|AssignOnActorEndOverlap _output_get (EventDispatchers|CreateEvent :!event Custom|OnActorEndOverlap_Event))
  (bind _asplayer_controller (Utilities|Casting|CastToPlayerController (Pawn|GetController (Variables|Default|GetPlayer))))
  (Variables|Default|SetPlayer%20Camera%20Manager (Variables|/Script/Engine.PlayerController|GetPlayerCameraManager _asplayer_controller)))

(fn GetInteractionActor
  (bind _sortedactors (Variables|Default|GetSortedActors))
  (if (Utilities|Array|IsValidIndex _sortedactors)
    (return true (Utilities|Array|Get(acopy) _sortedactors))
    (else
      (return false 0))))

(fn CalculateActorWeights
  (bind _weights (LocalVariables|GetWeights))
  (bind _l_sortedactors (LocalVariables|GetL_SortedActors))
  (bind _player_camera_manager (Variables|Default|GetPlayer%20Camera%20Manager))
  (bind _player (Variables|Default|GetPlayer))
  (bind _returnvalue (Camera|GetCameraRotation _player_camera_manager))
  (bind _returnvalue_2 (Transformation|GetActorLocation _player))
  (bind (_indexofminvalue _minvalue) (Math|Float|MinOfFloatArray _weights))
  (bind _output_get (LocalVariables|SetActors (Variables|Default|GetOverlappedActors)))
  (for (_array_element _array_index) _output_get
    (Utilities|Array|Add (LocalVariables|GetWeights) (+ (/ (Math|Vector|Distance(Vector) (Transformation|GetActorLocation _array_element) _returnvalue_2) 1.0) (* (- 1.0 (Math|Float|Max(Float) (Math|Vector|DotProduct (Math|Vector|Normalize (- (Transformation|GetActorLocation _array_element) (+ _returnvalue_2 (* (Math|Vector|GetRightVector _returnvalue) 5e+01) (* (Math|Vector|GetUpVector _returnvalue) 5e+01)))) (Math|Vector|GetForwardVector _returnvalue)) 0.0)) 1e+03))))
  (Utilities|Array|ReverseforEachLoop (LocalVariables|GetWeights)
    (:LoopBody
      (LocalVariables|SetL_MinWeightIndex _indexofminvalue)
      (Utilities|Array|Add (LocalVariables|GetSortedWeights) _minvalue)
      (Utilities|Array|Add (LocalVariables|GetL_SortedActors) (Utilities|Array|Get(acopy) (LocalVariables|GetActors) (LocalVariables|GetL_MinWeightIndex)))
      (Utilities|Array|RemoveIndex (LocalVariables|GetActors) (LocalVariables|GetL_MinWeightIndex))
      (Utilities|Array|RemoveIndex (LocalVariables|GetWeights) (LocalVariables|GetL_MinWeightIndex)))
    (:Completed
      (Variables|Default|SetSortedActors _l_sortedactors)
      (Class|BPIInteract|SetMarkerState(Message) (Utilities|Array|Get(acopy) _l_sortedactors) true)
      (Utilities|Array|RemoveIndex _l_sortedactors)
      (Class|BPIInteract|SetMarkerState(Message) (LocalVariables|GetL_SortedActors) false))))