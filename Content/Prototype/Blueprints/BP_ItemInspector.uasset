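; Item inspector actor that films a single item with a show-only orthographic scene capture for rotatable, zoomable inspection.
; SetActive attaches to the item's bounds center, moves its mesh to lighting channel 1 and derives zoom limits from bounds; deactivation restores channel 0 and reattaches to the owner.
; InspectionWindow events gate look and zoom input, which set targets that Tick interpolates into root rotation and ortho width.
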(event Custom|SetActive
  (params (isActive :type Boolean) (Item :type BP%20Base%20Item%20Object%20Reference))
  (bind _scenecapturecomponent2d (Variables|Default|GetSceneCaptureComponent2D))
  (bind _scenecapturecomponent2d_2 (Variables|Default|GetSceneCaptureComponent2D))
  (if isActive
    (Variables|Default|SetItem Item)
    (Transformation|AttachComponentToComponent (Variables|/Game/Prototype/Blueprints/BP_BaseItem.BP_BaseItem_C|GetBoundsCenter (Variables|Default|GetItem)) "None" "SnapToTarget" "SnapToTarget" "KeepWorld" true)
    (Rendering|SceneCapture|ClearShowOnlyComponents _scenecapturecomponent2d)
    (Rendering|SceneCapture|ShowOnlyComponent _scenecapturecomponent2d (Variables|/Game/Prototype/Blueprints/BP_BaseItem.BP_BaseItem_C|GetStaticMesh (Variables|Default|GetItem)))
    (Rendering|Components|SetLightingChannels (Variables|/Game/Prototype/Blueprints/BP_BaseItem.BP_BaseItem_C|GetStaticMesh (Variables|Default|GetItem)) false true false)
    (bind _output_get (Variables|CameraMoving|SetTargetRotation (Variables|/Script/Engine.SceneComponent|GetRelativeRotation (Variables|/Game/Prototype/Blueprints/BP_BaseItem.BP_BaseItem_C|GetInitRotation (Variables|Default|GetItem)))))
    (Transformation|SetActorRelativeRotation _output_get)
    (Variables|CameraMoving|SetMaxZoom (* (* (.SphereRadius (Collision|GetComponentBounds (Variables|/Game/Prototype/Blueprints/BP_BaseItem.BP_BaseItem_C|GetStaticMesh (Variables|Default|GetItem)))) 4.0) 0.5))
    (Variables|CameraMoving|SetZoomAlpha 1.0)
    (bind _output_get_2 (Variables|CameraMoving|SetMinZoom (* (.SphereRadius (Collision|GetComponentBounds (Variables|/Game/Prototype/Blueprints/BP_BaseItem.BP_BaseItem_C|GetStaticMesh (Variables|Default|GetItem)))) 4.0)))
    (bind _output_get_3 (Variables|CameraMoving|SetTargetZoom _output_get_2))
    (Variables|/Script/Engine.SceneCaptureComponent2D|SetOrthoWidth _scenecapturecomponent2d_2 _output_get_3)
    (Transformation|SetRelativeLocation _scenecapturecomponent2d_2 (Math|Vector|MakeVector (* _output_get_3 -1.0) 0.0 0.0) false false)
    (else
      (Components|Activation|SetActive (Variables|Default|GetSceneCaptureComponent2D) false false)
      (Rendering|Components|SetLightingChannels (Variables|/Game/Prototype/Blueprints/BP_BaseItem.BP_BaseItem_C|GetStaticMesh (Variables|Default|GetItem)) true false false)
      (Variables|Default|SetItem 0)
      (Transformation|AttachActorToActor (Components|GetOwner) "None" "KeepWorld" "KeepWorld" "KeepWorld" true))))

(event Custom|CanZoom
  (params (CanZoom :type Boolean))
  (Variables|CameraMoving|SetCan%20Zoom CanZoom))

(event Custom|TryRotate
  (params (TryRotate :type Boolean))
  (Variables|CameraMoving|SetTry%20Rotate TryRotate))

(event Input|EnhancedActionEvents|EnhancedInputActionIA_Zoom
  (params (ActionValue :type Float%20%28double-precision%29) (ElapsedSeconds :type Float%20%28double-precision%29) (TriggeredSeconds :type Float%20%28double-precision%29) (InputAction :type Input%20Action%20Object%20Reference :default "/Game/ThirdPerson/Input/Actions/IA_Zoom.IA_Zoom"))
  (if (Variables|CameraMoving|GetCan%20Zoom)
    (Variables|CameraMoving|SetZoomAlpha (Math|Float|Clamp(Float) (+ (* ActionValue (Variables|CameraMoving|Settings|GetZoomSense)) (Variables|CameraMoving|GetZoomAlpha))))
    (Variables|CameraMoving|SetTargetZoom (Math|Float|Lerp (Variables|CameraMoving|GetMaxZoom) (Variables|CameraMoving|GetMinZoom) (Variables|CameraMoving|GetZoomAlpha)))))

(event Input|EnhancedActionEvents|EnhancedInputActionIA_Look
  (params (ActionValue :type Vector%202D%20Structure) (ElapsedSeconds :type Float%20%28double-precision%29) (TriggeredSeconds :type Float%20%28double-precision%29) (InputAction :type Input%20Action%20Object%20Reference :default "/Game/ThirdPerson/Input/Actions/IA_Look.IA_Look"))
  (if (Variables|CameraMoving|GetTry%20Rotate)
    (Variables|CameraMoving|SetTargetRotation (Math|Rotator|MakeRotator 0.0 (Math|Float|Clamp(Float) (+ (.pitch (Variables|CameraMoving|GetTargetRotation)) (* (.y ActionValue) (Variables|CameraMoving|Settings|GetPitchRotationSense) -1.0)) -75.0 75.0) (+ (.yaw (Variables|CameraMoving|GetTargetRotation)) (* (.x ActionValue) (Variables|CameraMoving|Settings|GetYawRotationSense)))))))

(event EventTick
  (params (DeltaSeconds :type Float%20%28single-precision%29))
  (bind _scenecapturecomponent2d (Variables|Default|GetSceneCaptureComponent2D))
  (bind _defaultsceneroot (Variables|Default|GetDefaultSceneRoot))
  (Transformation|SetRelativeRotation _defaultsceneroot (Math|Interpolation|RInterpTo (Variables|/Script/Engine.SceneComponent|GetRelativeRotation _defaultsceneroot) (Variables|CameraMoving|GetTargetRotation) DeltaSeconds (Variables|CameraMoving|Settings|GetRotationInterpSpeed)) false false)
  (Variables|/Script/Engine.SceneCaptureComponent2D|SetOrthoWidth _scenecapturecomponent2d (Math|Interpolation|FInterpTo (Variables|/Script/Engine.SceneCaptureComponent2D|GetOrthoWidth _scenecapturecomponent2d) (Variables|CameraMoving|GetTargetZoom) DeltaSeconds (Variables|CameraMoving|Settings|GetZoomInterpSpeed))))

(event EventBeginPlay
  (bind _inspectionwindow (Variables|Default|GetInspectionWindow))
  (EventDispatchers|BindEventtoOnCanZoomInspection _inspectionwindow (delegate Custom|CanZoom))
  (EventDispatchers|BindEventtoOnTryRotateInspection _inspectionwindow (delegate Custom|TryRotate)))

(fn ConstructionScript)