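; BP_MyCharacter is a player character that detects nearby interactable actors and starts interactions with them.
; An InteractionSphere overlap checks for the BPI_Interact interface, toggles the actor's interact message and tracks it as the near interaction actor.
; The IA_Interact input calls StartInteractMessage on that actor; an Inspect result casts it to BP_BaseItem and fires the OnTryInspectionItem dispatcher.
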(event OnComponentBeginOverlap(InteractionSphere)
  (params (OverlappedComponent :type Primitive%20Component%20Object%20Reference) (OtherActor :type Actor%20Object%20Reference) (OtherComp :type Primitive%20Component%20Object%20Reference) (OtherBodyIndex :type Integer) (bFromSweep :type Boolean) (SweepResult :type Hit%20Result%20Structure%20%28by%20ref%29))
  (if (Utilities|DoesObjectImplementInterface OtherActor "/Game/Prototype/Blueprints/BPI_Interact.BPI_Interact_C")
    (Class|BPIInteract|SetInteractable(Message) OtherActor true)
    (Variables|Default|SetNearInteractionActor OtherActor)))

(event OnComponentEndOverlap(InteractionSphere)
  (params (OverlappedComponent :type Primitive%20Component%20Object%20Reference) (OtherActor :type Actor%20Object%20Reference) (OtherComp :type Primitive%20Component%20Object%20Reference) (OtherBodyIndex :type Integer))
  (if (Utilities|DoesObjectImplementInterface OtherActor "/Game/Prototype/Blueprints/BPI_Interact.BPI_Interact_C")
    (Class|BPIInteract|SetInteractable(Message) OtherActor false)
    (Variables|Default|SetNearInteractionActor 0)))

(event Input|EnhancedActionEvents|EnhancedInputActionIA_Interact
  (params (ActionValue :type Boolean) (ElapsedSeconds :type Float%20%28double-precision%29) (TriggeredSeconds :type Float%20%28double-precision%29) (InputAction :type Input%20Action%20Object%20Reference :default "/Game/ThirdPerson/Input/Actions/IA_Interact.IA_Interact"))
  (bind _nearinteractionactor (Variables|Default|GetNearInteractionActor)
    (:then
      (bind _interactiontype (Class|BPIInteract|StartInteract(Message) _nearinteractionactor))
      (switch Utilities|FlowControl|Switch|SwitchonEInteractionType _interactiontype
        (:NewEnumerator1
          (bind _asbp_base_item (Utilities|Casting|CastToBP_BaseItem _nearinteractionactor))
          (Default|CallOnTryInspectionItem _asbp_base_item))))
    (:else)))

(fn ConstructionScript
  (|CallParentFunction))