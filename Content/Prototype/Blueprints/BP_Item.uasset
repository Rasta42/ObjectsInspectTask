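; BP_Item is an interactable world item that supplies its name, description and collectible flag for inspection.
; SetInteractable swaps the icon material and toggles the button hint, while StartInteract returns a fixed enum value.
; SetCollectedState stores the flag, fires OnCollected (noted as a quest-system example), then hides the actor and disables its collision.
; Unless custom collision is set, the construction script makes mesh components overlap a custom trace channel.
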(event EventSetCollectedState
  (params (isCollected :type Boolean))
  (Variables|Default|SetIs%20Collected isCollected)
  ;[1 1 1] Example for quest system, but better will use item id
  (Default|CallOnCollected self)
  (Rendering|SetActorHiddenInGame true)
  (Collision|SetActorEnableCollision false))

(event EventSetInteractable
  (params (IsInteractable :type Boolean))
  (Rendering|Material|SetMaterial (Variables|Default|GetIcon) 0 (select IsInteractable "/Game/Prototype/Materials/M_InspectionItem_Inst.M_InspectionItem_Inst" "/Game/Prototype/Materials/M_ItemIcon_Inst.M_ItemIcon_Inst"))
  (Rendering|SetVisibility (Variables|Default|GetButtonHint) IsInteractable false))

(fn ConstructionScript
  (if (not (Variables|Default|GetisCustomCollision))
    (Collision|SetCollisionResponsetoChannel (Actor|GetComponentsByClass "/Script/Engine.MeshComponent") "ECC_GameTraceChannel1" "ECR_Overlap")))

(fn GetInspectionInfo
  (return (Variables|Default|GetisCollectible) (Variables|Default|GetName) (Variables|Default|GetDescription)))

(fn StartInteract
  (return "NewEnumerator1"))