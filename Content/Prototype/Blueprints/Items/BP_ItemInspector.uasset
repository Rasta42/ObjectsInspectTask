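; BP_ItemInspector runs the item inspection mode, showing a single BP_BaseItem through a scene capture and an inspection widget.
; Setup binds every item's interaction event and starts a timer that shows item markers near the player.
; Inspecting attaches the actor to the item, isolates it via show-only capture and lighting channels, and timer-interpolates rotation and orthographic zoom.
; Finishing restores player input and marks collectible items collected.
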(event Custom|InspectItem
  (params (Item :type BP%20Base%20Item%20Object%20Reference))
  (bind _playercontroller (Variables|Default|GetPlayerController))
  (bind _inspectionwindow (Variables|Default|GetInspectionWindow))
  (Input|DisableInput (Variables|Default|GetPlayerCharacter) _playercontroller)
  (Input|EnableInput _playercontroller)
  (CallFunction|SetActive true Item)
  (Default|SetInspectionState _inspectionwindow true Item)
  (Input|SetInputModeGameandUI (Variables|Default|GetPlayerController) _inspectionwindow "DoNotLock" false true))

(event Custom|ItemInspected
  (params (Item :type BP%20Base%20Item%20Object%20Reference))
  (bind _playercontroller (Variables|Default|GetPlayerController))
  (Input|EnableInput (Variables|Default|GetPlayerCharacter) _playercontroller)
  (Input|DisableInput _playercontroller)
  (Default|SetInspectionState (Variables|Default|GetInspectionWindow) false)
  (CallFunction|SetActive false)
  (Input|SetInputModeGameOnly (Variables|Default|GetPlayerController) true)
  (bind _iscollectible (Default|GetInspectionInfo Item))
  (if _iscollectible
    (Default|SetCollectedState Item true)))

(event Custom|SetActive
  (params (isActive :type Boolean) (Item :type BP%20Base%20Item%20Object%20Reference))
  (bind _scenecapturecomponent2d (Variables|Default|GetSceneCaptureComponent2D))
  (bind _scenecapturecomponent2d_2 (Variables|Default|GetSceneCaptureComponent2D))
  (if isActive
    (Variables|Default|SetItem Item)
    (Transformation|AttachComponentToComponent (Variables|/Game/Prototype/Blueprints/Items/BP_BaseItem.BP_BaseItem_C|GetBoundsCenter (Variables|Default|GetItem)) "None" "SnapToTarget" "SnapToTarget" "KeepWorld" true)
    (Rendering|SceneCapture|ClearShowOnlyComponents _scenecapturecomponent2d)
    (Rendering|SceneCapture|ShowOnlyComponent _scenecapturecomponent2d (Variables|/Game/Prototype/Blueprints/Items/BP_BaseItem.BP_BaseItem_C|GetStaticMesh (Variables|Default|GetItem)))
    (Rendering|Components|SetLightingChannels (Variables|/Game/Prototype/Blueprints/Items/BP_BaseItem.BP_BaseItem_C|GetStaticMesh (Variables|Default|GetItem)) false true false)
    (bind _output_get (Variables|CameraMoving|SetTargetRotation (Variables|/Script/Engine.SceneComponent|GetRelativeRotation (Variables|/Game/Prototype/Blueprints/Items/BP_BaseItem.BP_BaseItem_C|GetInitRotation (Variables|Default|GetItem)))))
    (Transformation|SetActorRelativeRotation _output_get)
    (Variables|CameraMoving|SetMaxZoom (* (* (.SphereRadius (Collision|GetComponentBounds (Variables|/Game/Prototype/Blueprints/Items/BP_BaseItem.BP_BaseItem_C|GetStaticMesh (Variables|Default|GetItem)))) 4.0) 0.5))
    (Variables|CameraMoving|SetZoomAlpha 1.0)
    (bind _output_get_2 (Variables|CameraMoving|SetMinZoom (* (.SphereRadius (Collision|GetComponentBounds (Variables|/Game/Prototype/Blueprints/Items/BP_BaseItem.BP_BaseItem_C|GetStaticMesh (Variables|Default|GetItem)))) 4.0)))
    (bind _output_get_3 (Variables|CameraMoving|SetTargetZoom _output_get_2))
    (Variables|/Script/Engine.SceneCaptureComponent2D|SetOrthoWidth _scenecapturecomponent2d_2 _output_get_3)
    (Transformation|SetRelativeLocation _scenecapturecomponent2d_2 (Math|Vector|MakeVector (* _output_get_3 -1.0) 0.0 0.0) false false)
    (bind _returnvalue (Utilities|Time|SetTimerbyEvent (EventDispatchers|CreateEvent :!event Custom|InspectorMovingUpdate) (Variables|Default|GetInspectorMovingDelta) true))
    (Variables|Default|SetInspectorTickTimer _returnvalue)
    (else
      (Components|Activation|SetActive (Variables|Default|GetSceneCaptureComponent2D) false false)
      (Rendering|Components|SetLightingChannels (Variables|/Game/Prototype/Blueprints/Items/BP_BaseItem.BP_BaseItem_C|GetStaticMesh (Variables|Default|GetItem)) true false false)
      (Variables|Default|SetItem 0)
      (Utilities|Time|ClearandInvalidateTimerbyHandle (Variables|Default|GetInspectorTickTimer)))))

(event Custom|InspectorMovingUpdate
  (bind _scenecapturecomponent2d (Variables|Default|GetSceneCaptureComponent2D))
  (bind _defaultsceneroot (Variables|Default|GetDefaultSceneRoot))
  (Transformation|SetRelativeRotation _defaultsceneroot (Math|Interpolation|RInterpTo (Variables|/Script/Engine.SceneComponent|GetRelativeRotation _defaultsceneroot) (Variables|CameraMoving|GetTargetRotation) (Variables|Default|GetInspectorMovingDelta) (Variables|CameraMoving|GetRotationInterpSpeed)) false false)
  (Variables|/Script/Engine.SceneCaptureComponent2D|SetOrthoWidth _scenecapturecomponent2d (Math|Interpolation|FInterpTo (Variables|/Script/Engine.SceneCaptureComponent2D|GetOrthoWidth _scenecapturecomponent2d) (Variables|CameraMoving|GetTargetZoom) (Variables|Default|GetInspectorMovingDelta) (Variables|CameraMoving|GetZoomInterpSpeed))))

(event Custom|AddRotation
  (params (Pitch :type Float%20%28double-precision%29) (Yaw :type Float%20%28double-precision%29))
  (Variables|CameraMoving|SetTargetRotation (Math|Rotator|MakeRotator 0.0 (Math|Float|Clamp(Float) (+ (.pitch (Variables|CameraMoving|GetTargetRotation)) Pitch) -75.0 75.0) (+ (.yaw (Variables|CameraMoving|GetTargetRotation)) Yaw))))

(event Custom|AddZoom
  (params (ZoomAlpha :type Float%20%28double-precision%29))
  (Variables|CameraMoving|SetZoomAlpha (Math|Float|Clamp(Float) (+ ZoomAlpha (Variables|CameraMoving|GetZoomAlpha))))
  (Variables|CameraMoving|SetTargetZoom (Math|Float|Lerp (Variables|CameraMoving|GetMaxZoom) (Variables|CameraMoving|GetMinZoom) (Variables|CameraMoving|GetZoomAlpha))))

(event Custom|Setup
  (bind _asplayer_controller (Utilities|Casting|CastToPlayerController (Pawn|GetController (Variables|Default|GetPlayerCharacter))))
  (bind _output_get (Variables|Default|SetPlayerController _asplayer_controller))
  (bind _returnvalue (UserInterface|CreateWidget "/Game/Prototype/Blueprints/UI/WBP_InspectionWindow.WBP_InspectionWindow_C" _output_get self))
  (bind _output_get_2 (Variables|Default|SetInspectionWindow _returnvalue))
  (Widget|SetVisibility _output_get_2 "Collapsed")
  (UserInterface|Viewport|AddtoViewport _output_get_2 666)
  (EventDispatchers|BindEventtoOnItemInspected _output_get_2 (EventDispatchers|CreateEvent :!event Custom|ItemInspected))
  (bind _outactors (Actor|GetAllActorsOfClass "/Game/Prototype/Blueprints/Items/BP_BaseItem.BP_BaseItem_C"))
  (Utilities|Set|AddItems (Variables|Default|GetAllItems) _outactors)
  (EventDispatchers|AssignOnIterracted _outactors (EventDispatchers|CreateEvent :!event Custom|InspectItem))
  (Utilities|Time|SetTimerbyEvent (EventDispatchers|CreateEvent :!event PlayerUpdate) (Variables|Default|GetPlayerUpdateDelta) true))

(fn ConstructionScript)

(fn AddNewItem
  (params (NewItem :type BP%20Base%20Item%20Object%20Reference%20%28by%20ref%29))
  (Utilities|Set|Add (Variables|Default|GetAllItems) NewItem)
  (EventDispatchers|BindEventtoOnIterracted NewItem (EventDispatchers|CreateEvent :!event Custom|InspectItem)))

(fn PlayerUpdate
  (bind _result (Utilities|Set|ToArray (Variables|Default|GetAllItems)))
  (for _array_element _result
    (Default|SetMarkerVisible _array_element (< (Transformation|GetDistanceTo _array_element (Variables|Default|GetPlayerCharacter)) (* (Variables|Default|GetMarkerDistance) 1e+02)))))