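; BP_BaseItem is a base interactable item that can be inspected and flagged as collectible, with a widget marker showing its interaction state.
; On BeginPlay it registers with the level's BP_ItemInspector, spawning one owned by the player character if none exists.
; Interaction and collection fire dispatchers, and collection also hides the actor and disables collision.
; The construction script centers BoundsCenter on the mesh bounds; capsule overlap only prints debug text.
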(event OnComponentBeginOverlap(InteractionCapsule)
  (params (OverlappedComponent :type Primitive%20Component%20Object%20Reference) (OtherActor :type Actor%20Object%20Reference) (OtherComp :type Primitive%20Component%20Object%20Reference) (OtherBodyIndex :type Integer) (bFromSweep :type Boolean) (SweepResult :type Hit%20Result%20Structure%20%28by%20ref%29))
  (Development|PrintString (Utilities|GetDisplayName OverlappedComponent)))

(event EventSetCollectedState
  (params (isCollected :type Boolean))
  (Variables|Proggres|SetIs%20Collected isCollected)
  ;[0 0 1] Коллбек для квестовой системы или чего то подобного
  (Default|CallOnCollected self)
  (Rendering|SetActorHiddenInGame true)
  (Collision|SetActorEnableCollision false))

(event EventBeginPlay
  (Variables|Default|SetMarkerWidget (.AsWBP%20Interaction%20Marker (Utilities|Casting|CastToWBP_InteractionMarker (UserInterface|GetWidget (Variables|Default|GetInteractionMarker)))))
  (bind _inspector (CallFunction|FindorCreateInspector))
  (Default|AddNewItem _inspector self))

(event EventSetMarkerState
  (params (InterractState :type EInteractionState%20Enum :default "NewEnumerator0"))
  (Default|SelectMarkerWidget (Variables|Default|GetMarkerWidget) InterractState))

(event EventSetMarkerVisible
  (params (IsVisible :type Boolean))
  (Rendering|SetVisibility (Variables|Default|GetInteractionMarker) IsVisible false))

(fn ConstructionScript
  (Transformation|SetWorldLocation (Variables|Default|GetBoundsCenter) (.Origin (Collision|GetComponentBounds (Variables|Default|GetStaticMesh))) false false))

(fn GetInspectionInfo
  (return (Variables|Default|GetisCollectible) (Variables|Default|GetName) (Variables|Default|GetDescription)))

(fn FindorCreateInspector
  (bind _returnvalue (Actor|GetActorOfClass "/Game/Prototype/Blueprints/Items/BP_ItemInspector.BP_ItemInspector_C"))
  (Utilities|IsValid _returnvalue
    (:Is%20Valid
      (return _returnvalue))
    (:Is%20Not%20Valid
      (bind _asbp_my_character (Utilities|Casting|CastToBP_MyCharacter (Game|Player|GetPlayerPawn 0)))
      (bind _returnvalue_2 (Game|SpawnActorfromClass "/Game/Prototype/Blueprints/Items/BP_ItemInspector.BP_ItemInspector_C" (Transformation|GetActorTransform _asbp_my_character) "AlwaysSpawn" "MultiplyWithRoot" _asbp_my_character _asbp_my_character _asbp_my_character))
      (Default|Setup _returnvalue_2)
      (return _returnvalue_2))))

(fn StartInteract
  ;[0 0 1] Need isBound check
  (Default|CallOnIterracted self)
  (return true))