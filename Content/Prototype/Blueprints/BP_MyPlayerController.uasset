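; Player controller that runs the item inspection mode for BP_MyCharacter.
; On possession it binds the character's inspection request, creates the HUD and spawns an item inspector attached to the pawn at an offset.
; An inspection request moves input from pawn to inspector and shows the inspection UI with a cursor.
; The inspection window's completion event restores game-only control and marks collectible items as collected.
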(event Custom|TryInspectionItem
  (params (Item :type BP%20Base%20Item%20Object%20Reference))
  (bind _self self)
  (bind _hud (Variables|Default|GetHUD))
  (bind _iteminspector (Variables|Default|GetItemInspector))
  (Input|DisableInput (Pawn|GetControlledPawn) _self)
  (Input|EnableInput _iteminspector _self)
  (Default|SetActive _iteminspector true Item)
  (Default|SetInspectionState _hud true Item)
  (Input|SetInputModeGameandUI self _hud "DoNotLock" false true)
  (Variables|Default|SetbShowMouseCursor true))

(event Custom|ItemInspected
  (params (Item :type BP%20Base%20Item%20Object%20Reference))
  (bind _self self)
  (bind _iteminspector (Variables|Default|GetItemInspector))
  (Input|EnableInput (Pawn|GetControlledPawn) _self)
  (Input|DisableInput _iteminspector _self)
  (Default|SetInspectionState (Variables|Default|GetHUD) false)
  (Default|SetActive _iteminspector false)
  (Input|SetInputModeGameOnly self true)
  (Variables|Default|SetbShowMouseCursor false)
  (bind _iscollectible (Default|GetInspectionInfo Item))
  (if _iscollectible
    (Default|SetCollectedState Item true)))

(event EventPossess
  (params (PossessedPawn :type Pawn%20Object%20Reference))
  (bind _returnvalue (Pawn|GetControlledPawn))
  (|CallParentFunction PossessedPawn)
  (bind _asbp_my_character (Utilities|Casting|CastToBP_MyCharacter PossessedPawn))
  (Utilities|FlowControl|Sequence
    (:then_0
      (EventDispatchers|BindEventtoOnTryInspectionItem _asbp_my_character (EventDispatchers|CreateEvent :!event Custom|TryInspectionItem)))
    (:then_1
      (bind _returnvalue_2 (UserInterface|CreateWidget "/Game/Prototype/UI/WBP_HUD.WBP_HUD_C"))
      (bind _output_get (Variables|Default|SetHUD _returnvalue_2))
      (UserInterface|Viewport|AddtoViewport _output_get 0)
      (EventDispatchers|BindEventtoOnItemInspected (Variables|/Game/Prototype/UI/WBP_HUD.WBP_HUD_C|GetWBP_InspectionWindow _output_get) (EventDispatchers|CreateEvent :!event Custom|ItemInspected)))
    (:then_2
      (bind _returnvalue_3 (Game|SpawnActorfromClass "/Game/Prototype/Blueprints/BP_ItemInspector.BP_ItemInspector_C" (|CalculateRelativeTransform _returnvalue "0.000000,0.000000,300.000000") "Undefined" "MultiplyWithRoot" _returnvalue (Variables|/Game/Prototype/UI/WBP_HUD.WBP_HUD_C|GetWBP_InspectionWindow (Variables|Default|GetHUD)) _returnvalue))
      (bind _output_get_2 (Variables|Default|SetItemInspector _returnvalue_3))
      (Transformation|AttachActorToActor _output_get_2 (Pawn|GetControlledPawn) "None" "KeepWorld" "KeepWorld" "KeepWorld" true))))

(event EventUnPossess
  (params (UnpossessedPawn :type Pawn%20Object%20Reference))
  (|CallParentFunction UnpossessedPawn)
  (bind _asbp_my_character (Utilities|Casting|CastToBP_MyCharacter UnpossessedPawn))
  (EventDispatchers|UnbindEventfromOnTryInspectionItem _asbp_my_character (EventDispatchers|CreateEvent :!event Custom|TryInspectionItem)))

(fn ConstructionScript)